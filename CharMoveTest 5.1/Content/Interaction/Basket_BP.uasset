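; Basket actor that tips and shakes a basket and handles a transition to level stage1_2.
; BasketRotationChange drives the basket's position and pitch with a timeline, then starts a loop that picks right-left or left-right pitch timelines from direction flags.
; StudioTeleport enables physics on PlayerSit and opens the level after a short delay.
; The center-to-right swing and player relocation are unconnected.
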(event EventStudioTeleport
  (Physics|SetSimulatePhysics (Variables|Default|GetPlayerSit) true)
  (Utilities|FlowControl|Delay 1.0)
  (Game|OpenLevel(byName) "stage1_2"))

(event EventBasketRotationChange
  (Development|PrintString "Hello")
  (Utilities|FlowControl|Delay 0.05)
  (bind (_direction _xlocation _zlocation _yrotation) (Timeline|타임라인 Play)
    (:Update
      (Transformation|SetRelativeLocationAndRotation (Variables|Default|GetBasket) (Math|Vector|MakeVector _xlocation 0.0 _zlocation) (Math|Rotator|MakeRotator 0.0 _yrotation 0.0) false false))
    (:Finished
      (Class|Basket|BasketShakeLoop))))

(event EventBasketShakeLoop
  (for _index (range (Variables|Default|GetLoop) 100)
    (Utilities|FlowControl|Delay 0.4)
    (if (Variables|Default|GetisRight?)
      (Development|PrintString "R->L")
      (bind _새_트랙_0 (Timeline|Right->Left PlayFromStart)
        (:Update
          (Transformation|AddLocalRotation (Variables|Default|GetBasket) (Math|Rotator|MakeRotator 0.0 _새_트랙_0 0.0) false false)
          (Transformation|AddLocalRotation (Variables|Default|GetBasket) (Math|Rotator|MakeRotator 0.0 _새_트랙_0 0.0) false false)
          (Variables|Default|SetisLeft? true)
          (Variables|Default|SetLoop (+ (Variables|Default|GetLoop) 1))))
      (elif (Variables|Default|GetisLeft?)
        (Development|PrintString "L->R")
        (bind _새_트랙_0_2 (Timeline|Left->Right PlayFromStart)
          (:Update
            (Transformation|AddLocalRotation (Variables|Default|GetBasket) (Math|Rotator|MakeRotator 0.0 _새_트랙_0_2 0.0) false false)
            (Transformation|AddLocalRotation (Variables|Default|GetBasket) (Math|Rotator|MakeRotator 0.0 _새_트랙_0_2 0.0) false false)
            (Variables|Default|SetisRight? true)
            (Variables|Default|SetLoop (+ (Variables|Default|GetLoop) 1))))))))

(fn ConstructionScript)