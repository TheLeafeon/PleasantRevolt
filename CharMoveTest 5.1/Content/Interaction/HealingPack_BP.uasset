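; Healing pickup Blueprint that restores the player's health when touched.
; On static mesh overlap it casts the other actor to BP_PlayerableCharacter and reads its current and max HP.
; If the player is below max HP, it adds a fixed amount of HP and destroys itself; at full health the pack stays in place.
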(event OnComponentBeginOverlap(StaticMesh)
  (params (OverlappedComponent :type Primitive%20Component%20Object%20Reference) (OtherActor :type Actor%20Object%20Reference) (OtherComp :type Primitive%20Component%20Object%20Reference) (OtherBodyIndex :type Integer) (bFromSweep :type Boolean) (SweepResult :type Hit%20Result%20Structure%20%28by%20ref%29))
  (bind _asbp_playerable_character (Utilities|Casting|CastToBP_PlayerableCharacter OtherActor))
  (bind _output_get (Variables|Default|SetPlayer _asbp_playerable_character))
  (bind _returnvalue (Class|PlayerableCharacter|GetPlayerMaxHP _output_get))
  (Variables|Default|SetPlayerMaxHp _returnvalue)
  (bind _returnvalue_2 (Class|PlayerableCharacter|GetPlayerHP (Variables|Default|GetPlayer)))
  (if (< _returnvalue_2 (Variables|Default|GetPlayerMaxHp))
    (Class|PlayerableCharacter|IncreasePlayerHP (Variables|Default|GetPlayer) 1.0)
    (Actor|DestroyActor)))

(fn ConstructionScript)