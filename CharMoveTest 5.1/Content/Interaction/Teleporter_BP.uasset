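; Teleporter Blueprint that moves the player pawn when it enters the TeleportIn volume, behind a Darkness screen widget.
; Begin overlap by any actor creates and shows UMG_Darkness if none is referenced, then, only for the player pawn, calls ActorTeleport after a short delay.
; The player's end overlap clears the widget reference, re-arming the trigger without removing the widget here.
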(event OnComponentBeginOverlap(TeleportIn)
  (params (OverlappedComponent :type Primitive%20Component%20Object%20Reference) (OtherActor :type Actor%20Object%20Reference) (OtherComp :type Primitive%20Component%20Object%20Reference) (OtherBodyIndex :type Integer) (bFromSweep :type Boolean) (SweepResult :type Hit%20Result%20Structure%20%28by%20ref%29))
  (if (not (Utilities|IsValid (Variables|Default|GetDarkness)))
    (bind _returnvalue (UserInterface|CreateWidget "/Game/Interaction/UI/UMG_Darkness.UMG_Darkness_C" (Game|GetPlayerController 0)))
    (bind _output_get (Variables|Default|SetDarkness _returnvalue))
    (UserInterface|Viewport|AddtoViewport _output_get 0)
    (if (== OtherActor (Game|Player|GetPlayerPawn 0))
      (Utilities|FlowControl|Delay 0.1)
      (Class|Teleporter|ActorTeleport OtherActor))))

(event OnComponentEndOverlap(TeleportIn)
  (params (OverlappedComponent :type Primitive%20Component%20Object%20Reference) (OtherActor :type Actor%20Object%20Reference) (OtherComp :type Primitive%20Component%20Object%20Reference) (OtherBodyIndex :type Integer))
  (if (== OtherActor (Game|Player|GetPlayerPawn 0))
    (Variables|Default|SetDarkness 0)))

(event EventBeginPlay)

(event EventTick
  (params (DeltaSeconds :type Float%20%28single-precision%29)))

(fn ConstructionScript)