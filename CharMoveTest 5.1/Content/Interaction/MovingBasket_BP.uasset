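; MovingBasket_BP is an interaction actor for a basket that can be shaken and can send the game to another level.
; ShakeBasket plays a timeline that drives the basket component's world location and rotation from per-axis tracks.
; GotoStudioLevel opens stage1_2_reMonster; neither event is called within this graph.
; The box overlap only latches a FirstIn flag when the player first enters, without triggering either event.
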(event OnComponentBeginOverlap(Box)
  (params (OverlappedComponent :type Primitive%20Component%20Object%20Reference) (OtherActor :type Actor%20Object%20Reference) (OtherComp :type Primitive%20Component%20Object%20Reference) (OtherBodyIndex :type Integer) (bFromSweep :type Boolean) (SweepResult :type Hit%20Result%20Structure%20%28by%20ref%29))
  (if (== (== OtherActor (Game|GetPlayerCharacter 0)) (not (Variables|Default|GetfirstIn)))
    (Variables|Default|SetfirstIn true)))

(event EventShakeBasket
  (bind (_direction _locationx _locationy _locationz _rotationx _rotationy _rotationz) (Timeline|타임라인 Play)
    (:Update
      (Transformation|SetWorldLocationAndRotation (Variables|Default|GetBasketComp) (Math|Vector|MakeVector _locationx _locationy _locationz) (Math|Rotator|MakeRotator _rotationx _rotationy _rotationz) false false))))

(event EventGotoStudioLevel
  (Game|OpenLevel(byName) "stage1_2_reMonster"))

(fn ConstructionScript)