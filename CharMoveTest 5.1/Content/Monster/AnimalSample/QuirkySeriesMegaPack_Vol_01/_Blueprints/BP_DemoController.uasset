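; Showcase controller for the animal sample pack that lets the player browse animals and their animations.
; On BeginPlay it spawns every AnimalsBP class at its own transform, and N/M cycle which one is visible by toggling root visibility.
; Z/X step through the ActiveAnimation enum, which indexes each animal's GetAnimationsMessage list to play that clip on all spawned meshes.
; UpdateText refreshes the animal and animation labels with key hints.
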(event EventBeginPlay
  (bind _activeanimation (Variables|Default|GetactiveAnimation))
  (bind _animalsbp (Variables|Default|GetanimalsBP))
  (Input|EnableInput (Game|GetPlayerController 0))
  ;[1 1 1] Spawn and append into animals array
  (for (_ _array_index) _animalsbp
    (bind _returnvalue (Game|SpawnActorfromClass (Utilities|Array|Get(acopy) _animalsbp _array_index) (Transformation|GetActorTransform) "Undefined" 0 0))
    (Utilities|Array|AppendArray (Variables|Default|GetspawnedAnimals) (Utilities|Array|MakeArray _returnvalue))
    ;[1 1 1] Enable input for first animal
    (if (Math|Conversions|ToBoolean(Integer) _array_index)
      (Rendering|ToggleVisibility (Variables|/Script/Engine.Actor|GetRootComponent _returnvalue) false))
    (Input|EnableInput _returnvalue (Game|GetPlayerController 0))
    (CallFunction|UpdateText)
    ;[1 1 1] Cycle animation
    (for _array_element (Variables|Default|GetspawnedAnimals)
      (Components|Animation|SetAnimationMode (Actor|GetComponentbyClass _array_element "/Script/Engine.SkeletalMeshComponent") "AnimationBlueprint")
      (bind _newparam (Class|Object|GetAnimations(Message) _array_element))
      (Components|Animation|PlayAnimation (Actor|GetComponentbyClass _array_element "/Script/Engine.SkeletalMeshComponent") (Utilities|Array|Get(acopy) _newparam (Math|Conversions|ToInteger(Byte) _activeanimation)) (!= _activeanimation (Utilities|Enum|Literalenum)))
      (Rendering|SetVisibility (Variables|Default|GetAnimalName) true false)
      (Rendering|SetVisibility (Variables|Default|GetInstruction) false false))))

(event Input|KeyboardEvents|N
  (params (Key :type Key%20Structure))
  (bind _spawnedanimals (Variables|Default|GetspawnedAnimals))
  (bind _activeanimation (Variables|Default|GetactiveAnimation))
  (:Released
    ;[1 1 1] Hide current animal and disable its input
    (Rendering|ToggleVisibility (Variables|/Script/Engine.Actor|GetRootComponent (Utilities|Array|Get(acopy) (Variables|Default|GetspawnedAnimals) (Variables|Default|GetanimalIndex))) false)
    ;[1 1 1] Show next/prev animal and enable its input
    (bind _result (Math|Integer|DecrementInt (Variables|Default|GetanimalIndex))
      (:%20%20
        (Math|Integer|CompareInt _result
          (:>
            _)
          (:==
            _)
          (:<
            (bind _result_2 (Math|Integer|DecrementInt (Utilities|Array|Length _spawnedanimals))
              (:%20%20
                (Variables|Default|SetanimalIndex _result_2)))))
        (Rendering|ToggleVisibility (Variables|/Script/Engine.Actor|GetRootComponent (Utilities|Array|Get(acopy) _spawnedanimals (Variables|Default|GetanimalIndex))) false)
        (CallFunction|UpdateText)
        ;[1 1 1] Cycle animation
        (for _array_element (Variables|Default|GetspawnedAnimals)
          (Components|Animation|SetAnimationMode (Actor|GetComponentbyClass _array_element "/Script/Engine.SkeletalMeshComponent") "AnimationBlueprint")
          (bind _newparam (Class|Object|GetAnimations(Message) _array_element))
          (Components|Animation|PlayAnimation (Actor|GetComponentbyClass _array_element "/Script/Engine.SkeletalMeshComponent") (Utilities|Array|Get(acopy) _newparam (Math|Conversions|ToInteger(Byte) _activeanimation)) (!= _activeanimation (Utilities|Enum|Literalenum)))
          (Rendering|SetVisibility (Variables|Default|GetAnimalName) true false)
          (Rendering|SetVisibility (Variables|Default|GetInstruction) false false))))))

(event Input|KeyboardEvents|M
  (params (Key :type Key%20Structure))
  (bind _spawnedanimals (Variables|Default|GetspawnedAnimals))
  (bind _activeanimation (Variables|Default|GetactiveAnimation))
  (:Released
    ;[1 1 1] Hide current animal and disable its input
    (Rendering|ToggleVisibility (Variables|/Script/Engine.Actor|GetRootComponent (Utilities|Array|Get(acopy) (Variables|Default|GetspawnedAnimals) (Variables|Default|GetanimalIndex))) false)
    ;[1 1 1] Show next/prev animal and enable its input
    (bind _result (Math|Integer|IncrementInt (Variables|Default|GetanimalIndex))
      (:%20%20
        (Math|Integer|CompareInt _result (Utilities|Array|Length _spawnedanimals)
          (:>
            (Variables|Default|SetanimalIndex 0 :!label _label))
          (:==
            (goto _label))
          (:<
            _))
        (Rendering|ToggleVisibility (Variables|/Script/Engine.Actor|GetRootComponent (Utilities|Array|Get(acopy) _spawnedanimals (Variables|Default|GetanimalIndex))) false)
        (CallFunction|UpdateText)
        ;[1 1 1] Cycle animation
        (for _array_element (Variables|Default|GetspawnedAnimals)
          (Components|Animation|SetAnimationMode (Actor|GetComponentbyClass _array_element "/Script/Engine.SkeletalMeshComponent") "AnimationBlueprint")
          (bind _newparam (Class|Object|GetAnimations(Message) _array_element))
          (Components|Animation|PlayAnimation (Actor|GetComponentbyClass _array_element "/Script/Engine.SkeletalMeshComponent") (Utilities|Array|Get(acopy) _newparam (Math|Conversions|ToInteger(Byte) _activeanimation)) (!= _activeanimation (Utilities|Enum|Literalenum)))
          (Rendering|SetVisibility (Variables|Default|GetAnimalName) true false)
          (Rendering|SetVisibility (Variables|Default|GetInstruction) false false))))))

(event Input|KeyboardEvents|Z
  (params (Key :type Key%20Structure))
  (:Released
    ;[1 1 1] Update animal and animation text
    (Math|Integer|CompareInt (Math|Conversions|ToInteger(Byte) (Variables|Default|GetactiveAnimation))
      (:>
        (bind _result (Math|Integer|DecrementInt (Math|Conversions|ToInteger(Byte) (Variables|Default|GetactiveAnimation)))
          (:%20%20
            (Variables|Default|SetactiveAnimation (Utilities|Enum|ByteToEnumObject (Math|Conversions|ToByte(Integer) _result))))))
      (:==
        (Variables|Default|SetactiveAnimation (Utilities|Enum|ByteToEnumObject (Math|Conversions|ToByte(Integer) (- (|GetNumEnumEntries) 1))) :!label _label))
      (:<
        (goto _label)))
    (CallFunction|UpdateText)
    ;[1 1 1] Cycle animation
    (for _array_element (Variables|Default|GetspawnedAnimals)
      (Components|Animation|SetAnimationMode (Actor|GetComponentbyClass _array_element "/Script/Engine.SkeletalMeshComponent") "AnimationBlueprint")
      (bind _newparam (Class|Object|GetAnimations(Message) _array_element))
      (Components|Animation|PlayAnimation (Actor|GetComponentbyClass _array_element "/Script/Engine.SkeletalMeshComponent") (Utilities|Array|Get(acopy) _newparam (Math|Conversions|ToInteger(Byte) (Variables|Default|GetactiveAnimation))) (!= (Variables|Default|GetactiveAnimation) (Utilities|Enum|Literalenum)))
      (Rendering|SetVisibility (Variables|Default|GetAnimalName) true false)
      (Rendering|SetVisibility (Variables|Default|GetInstruction) false false))))

(event Input|KeyboardEvents|X
  (params (Key :type Key%20Structure))
  (:Released
    ;[1 1 1] Update animal and animation text
    (Math|Integer|CompareInt (Math|Conversions|ToInteger(Byte) (Variables|Default|GetactiveAnimation)) (- (|GetNumEnumEntries) 1)
      (:>
        (Variables|Default|SetactiveAnimation 0 :!label _label))
      (:==
        (goto _label))
      (:<
        (bind _result (Math|Integer|IncrementInt (Math|Conversions|ToInteger(Byte) (Variables|Default|GetactiveAnimation)))
          (:%20%20
            (Variables|Default|SetactiveAnimation (Utilities|Enum|ByteToEnumObject (Math|Conversions|ToByte(Integer) _result)))))))
    (CallFunction|UpdateText)
    ;[1 1 1] Cycle animation
    (for _array_element (Variables|Default|GetspawnedAnimals)
      (Components|Animation|SetAnimationMode (Actor|GetComponentbyClass _array_element "/Script/Engine.SkeletalMeshComponent") "AnimationBlueprint")
      (bind _newparam (Class|Object|GetAnimations(Message) _array_element))
      (Components|Animation|PlayAnimation (Actor|GetComponentbyClass _array_element "/Script/Engine.SkeletalMeshComponent") (Utilities|Array|Get(acopy) _newparam (Math|Conversions|ToInteger(Byte) (Variables|Default|GetactiveAnimation))) (!= (Variables|Default|GetactiveAnimation) (Utilities|Enum|Literalenum)))
      (Rendering|SetVisibility (Variables|Default|GetAnimalName) true false)
      (Rendering|SetVisibility (Variables|Default|GetInstruction) false false))))

(fn ConstructionScript)

(fn UpdateText
  ;[1 1 1] Update animal and animation name
  (Rendering|Components|TextRender|SetText (Variables|Default|GetAnimalName) (Utilities|Text|ToText(String) (Utilities|String|Append (Utilities|String|RightChop (Utilities|GetDisplayName (Utilities|Array|Get(acopy) (Variables|Default|GetspawnedAnimals) (Variables|Default|GetanimalIndex))) 3) " - [N/M] to change")))
  (Rendering|Components|TextRender|SetText (Variables|Default|GetAnimationName) (Utilities|Text|ToText(String) (Utilities|String|Append (Utilities|String|EnumtoString (Variables|Default|GetactiveAnimation)) " - [Z/X] to change"))))