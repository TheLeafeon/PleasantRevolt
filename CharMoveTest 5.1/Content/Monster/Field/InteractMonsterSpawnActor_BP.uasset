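; Field monster-encounter actor that drives a door, a ladder and a weapon reward around a battle.
; BattleStart reverses a timeline to lower the door; BattleEnd animates the ladder's height at hard-coded world coordinates while playing the door timeline forward.
; SetObj supplies the Door and Ladder references.
; GiveWeapontoPlayer passes the Weapon to GISSPlayer and calls AddWeapons on the player character; an older GameMode SpawnWeapon path is disconnected.
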(event EventBeginPlay)

(event EventBattleStart
  (bind _z (Timeline|타임라인 Reverse) ; 내려갈때
    (:Update
      (bind _asdoor_2 (Utilities|Casting|CastToDoor_2 (Variables|Default|GetDoor)))
      (Default|DoorMove _asdoor_2 _z))))

(event EventBattleEnd
  (bind _asladder_long (Utilities|Casting|CastToLadder_Long (Variables|Default|GetLadder)))
  (Transformation|SetActorLocation _asladder_long "3636.000000,130.000000,-4820.000000" false false)
  (bind _z (Timeline|타임라인_0 Play)
    (:Update
      (Transformation|SetActorLocation _asladder_long (Math|Vector|MakeVector 3636.0 1.3e+02 _z) false false)
      (bind _z_2 (Timeline|타임라인 Play) ; 내려갈때
        (:Update
          (bind _asdoor_2 (Utilities|Casting|CastToDoor_2 (Variables|Default|GetDoor)))
          (Default|DoorMove _asdoor_2 _z_2))))))

(event EventGiveWeapontoPlayer
  (Class|GISSPlayer|GetWeapon (Subsystems|GetGISSPlayer) (Variables|Default|GetWeapon))
  (bind _asbp_playerable_character (Utilities|Casting|CastToBP_PlayerableCharacter (Game|Player|GetPlayerPawn 0)))
  (Class|PlayerableCharacter|AddWeapons _asbp_playerable_character))

(fn ConstructionScript)

(fn SetObj
  (params (Ladder :type Actor%20Object%20Reference) (Door :type Actor%20Object%20Reference))
  (Variables|Default|SetLadder Ladder)
  (Variables|Default|SetDoor Door))