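; FieldArea_BP is a monster field area that moves its linked doors when the battle there ends.
; SetObj registers one door and SetObj2 registers two, recording the count in SetObjNum.
; BattleEnd switches on that count and plays the matching timeline, passing its Z track to DoorMove on each Door_2, marked in comments as the downward movement.
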(event EventBattleEnd
  (switch int (Variables|Default|GetSetObjNum)
    (:1
      (bind _z (Timeline|타임라인 Play) ; 내려갈때
        (:Update
          (bind _asdoor_2 (Utilities|Casting|CastToDoor_2 (Variables|Default|GetDoor)))
          (Default|DoorMove _asdoor_2 _z))))
    (:2
      (bind _z_2 (Timeline|타임라인_0 Play) ; 내려갈때
        (:Update
          (bind _asdoor_2_2 (Utilities|Casting|CastToDoor_2 (Variables|Default|GetDoor)))
          (Default|DoorMove _asdoor_2_2 _z_2)
          (bind _asdoor_2_3 (Utilities|Casting|CastToDoor_2 (Variables|Default|GetDoor2)))
          (Default|DoorMove _asdoor_2_3 _z_2))))))

(fn ConstructionScript)

(fn SetObj
  (params (Door :type Actor%20Object%20Reference))
  (Variables|Default|SetSetObjNum 1)
  (Variables|Default|SetDoor Door))

(fn SetObj2
  (params (Door1 :type Actor%20Object%20Reference) (Door2 :type Actor%20Object%20Reference))
  (Variables|Default|SetSetObjNum 2)
  (Variables|Default|SetDoor Door1)
  (Variables|Default|SetDoor2 Door2))