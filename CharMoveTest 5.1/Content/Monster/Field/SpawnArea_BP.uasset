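; Monster field spawn area that calls MonsterSpawn when something begins overlapping its CollisionBox, with no filter on the overlapping actor.
; Spawning requires either the IsBeginOverlapMonsterSpawn flag or MyAreaClear, which Tick copies from the linked MyFieldArea's AreaClear.
; FirstIn blocks later overlaps once a spawn fires, but both Sequence branches can spawn on the same overlap if both conditions hold.
; Debug strings print on overlap and spawn.
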(event OnComponentBeginOverlap(CollisionBox)
  (params (OverlappedComponent :type Primitive%20Component%20Object%20Reference) (OtherActor :type Actor%20Object%20Reference) (OtherComp :type Primitive%20Component%20Object%20Reference) (OtherBodyIndex :type Integer) (bFromSweep :type Boolean) (SweepResult :type Hit%20Result%20Structure%20%28by%20ref%29))
  (if (not (Variables|Default|GetfirstIn))
    (Development|PrintString "Overlap")
    (Utilities|FlowControl|Sequence
      (:then_0
        (if (Variables|Default|GetisBeginOverlapMonsterSpawn)
          (Variables|Default|SetfirstIn true)
          (Class|SpawnArea|MonsterSpawn)
          (Development|PrintString "OverlapSpawn")))
      (:then_1
        (if (Variables|Default|GetmyAreaClear)
          (Variables|Default|SetfirstIn true)
          (Class|SpawnArea|MonsterSpawn)
          (Development|PrintString "FieldClearSpawn"))))))

(event EventTick
  (params (DeltaSeconds :type Float%20%28single-precision%29))
  (bind _myfieldarea (Variables|Default|GetMyFieldArea))
  (Utilities|IsValid _myfieldarea
    (:Is%20Valid
      (Variables|Default|SetmyAreaClear (Variables|/Script/CharMoveTest.FieldArea|GetAreaClear _myfieldarea)))))

(fn ConstructionScript)