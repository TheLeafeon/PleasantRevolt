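; GirlDoll monster Blueprint that handles the doll's attack effect, knockback, damage and procedural wobble motion.
; While not readying an attack, Tick uses a delay, direction flags and center/right/left timelines to rock the static mesh's pitch side to side.
; Custom events spawn an explosion at the attack box, launch the doll away from the player, damage the player with MonsterPower and reset the mesh upright for attacks.
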(event EventGirlDollAttackSetMotion
  (bind _staticmesh (Variables|Default|GetStaticMesh))
  (bind _returnvalue (Transformation|GetWorldRotation _staticmesh))
  ;[1 1 1] 공격 모션 나올때 Rotation 변경
  (Variables|Default|SetisCenter? true)
  (Transformation|SetWorldRotation (Variables|Default|GetStaticMesh) (Math|Rotator|MakeRotator (.roll _returnvalue) 0.0 (.yaw _returnvalue)) false false))

(event Collision|EventActorBeginOverlap
  (params (OtherActor :type Actor%20Object%20Reference)))

(event EventTick
  (params (DeltaSeconds :type Float%20%28single-precision%29))
  ;[1 1 1] 점프 테스트
  (if (not (Variables|Default|GetisAttackReady))
    (Utilities|FlowControl|Delay 0.9)
    (if (Variables|Default|GetisCenter?)
      (bind _center__right (Timeline|CenterTimeLine PlayFromStart)
        (:Update
          (Transformation|AddLocalRotation (Variables|Default|GetStaticMesh) (Math|Rotator|MakeRotator 0.0 _center__right 0.0) false false)
          (Variables|Default|SetisCenter? false)
          (Variables|Default|SetisRight? true)))
      (elif (Variables|Default|GetisRight?)
        (bind _right__left (Timeline|RightTimeLine PlayFromStart)
          (:Update
            (Transformation|AddLocalRotation (Variables|Default|GetStaticMesh) (Math|Rotator|MakeRotator 0.0 _right__left 0.0) false false)
            (Transformation|AddLocalRotation (Variables|Default|GetStaticMesh) (Math|Rotator|MakeRotator 0.0 _right__left 0.0) false false)
            (Variables|Default|SetisRight? false)
            (Variables|Default|SetisLeft? true)))
        (elif (Variables|Default|GetisLeft?)
          (bind _left__right (Timeline|LeftTimeLine PlayFromStart)
            (:Update
              (Transformation|AddLocalRotation (Variables|Default|GetStaticMesh) (Math|Rotator|MakeRotator 0.0 _left__right 0.0) false false)
              (Transformation|AddLocalRotation (Variables|Default|GetStaticMesh) (Math|Rotator|MakeRotator 0.0 _left__right 0.0) false false)
              (Variables|Default|SetisLeft? false)
              (Variables|Default|SetisRight? true))))))))

(event EventGirlDollApplyDamageEvent
  ;[1 1 1] 플레이어에게 데미지 주기
  (bind _asbp_playerable_character (Utilities|Casting|CastToBP_PlayerableCharacter (Game|GetPlayerCharacter 0)))
  (Game|Damage|ApplyDamage _asbp_playerable_character (Variables|Default|GetMonster_Power) 0 0))

(event EventGirlDollAttackEffect
  ;[1 1 1] 공격시 파티클 생성
  (Effects|SpawnEmitteratLocation "/Game/StarterContent/Particles/P_Explosion.P_Explosion" (Transformation|GetWorldLocation (Variables|Default|GetAttackRangeBox))))

(event EventGirlDollKnockBack
  ;[1 1 1] 넉백 밀려나는 거리 문제있음, 밀려나면 Attack 중단 필요
  (Character|LaunchCharacter (* (Math|Vector|GetUnitDirection(Vector) (Transformation|GetActorLocation (Game|GetPlayerCharacter 0)) (Transformation|GetActorLocation)) (Math|Conversions|ToVector(Float) 3e+03)) false false))

(event EventBeginPlay)

(fn ConstructionScript)