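; FieldMonster_DoveDoll_BP is the dove doll field monster, with events for shooting, hit feedback, sounds and appearance effects.
; Fire spawns FPSProjectile_BP at the FirePoint transform, and another event records the head location and actor rotation.
; Unless the monster is dead, hits swap three mesh material slots to a hit material, blink HitParam, then restore the originals.
; A short-lived particle marks its appearance, and audio components play hit and death sounds.
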(event Custom|커스텀이벤트
  ;[1 1 1] 발사 위치
  (Variables|Default|SetDoveDollHeadLocation (Transformation|GetWorldLocation (Variables|Default|GetDoveDollHead)))
  (Variables|Default|SetDoveDollHeadRotation (Transformation|GetActorRotation)))

(event EventFire
  ;[1 1 1] 파이어
  (Game|SpawnActorfromClass "/Game/Monster/BP/FPSProjectile_BP.FPSProjectile_BP_C" (Transformation|GetWorldTransform (Variables|Default|GetFirePoint)) "Undefined" 0 0))

(event EventDoveDollHitMaterial
  (if (not (Variables|Default|GetisDie))
    ;[1 1 1] 흰색 길게
    (Utilities|FlowControl|Sequence
      (:then_0
        (Rendering|Material|SetMaterial (Variables|Character|GetMesh) 0 "/Game/Monster/Material/FieldMonster_material_Hit.FieldMonster_material_Hit")
        (Utilities|FlowControl|Delay 0.3)
        ;[1 1 1] 빨간색 깜빡
        (Rendering|Material|SetScalarParameterValueonMaterials (Variables|Character|GetMesh) "HitParam" 0.0)
        (Utilities|FlowControl|Delay 0.1)
        (Rendering|Material|SetScalarParameterValueonMaterials (Variables|Character|GetMesh) "HitParam" 1.0)
        (Utilities|FlowControl|Delay 0.1)
        (Rendering|Material|SetMaterial (Variables|Character|GetMesh) 0 "/Game/Object/animal/material/dove_material.dove_material"))
      (:then_1
        (Rendering|Material|SetMaterial (Variables|Character|GetMesh) 1 "/Game/Monster/Material/FieldMonster_material_Hit.FieldMonster_material_Hit")
        (Utilities|FlowControl|Delay 0.3)
        (Rendering|Material|SetScalarParameterValueonMaterials (Variables|Character|GetMesh) "HitParam" 0.0)
        (Utilities|FlowControl|Delay 0.1)
        (Rendering|Material|SetScalarParameterValueonMaterials (Variables|Character|GetMesh) "HitParam" 1.0)
        (Utilities|FlowControl|Delay 0.1)
        (Rendering|Material|SetMaterial (Variables|Character|GetMesh) 1 "/Game/Object/animal/material/cotton_animal_material.cotton_animal_material"))
      (:then_2
        (Rendering|Material|SetMaterial (Variables|Character|GetMesh) 2 "/Game/Monster/Material/FieldMonster_material_Hit.FieldMonster_material_Hit")
        (Utilities|FlowControl|Delay 0.3)
        (Rendering|Material|SetScalarParameterValueonMaterials (Variables|Character|GetMesh) "HitParam" 0.0)
        (Utilities|FlowControl|Delay 0.1)
        (Rendering|Material|SetScalarParameterValueonMaterials (Variables|Character|GetMesh) "HitParam" 1.0)
        (Utilities|FlowControl|Delay 0.1)
        (Rendering|Material|SetMaterial (Variables|Character|GetMesh) 2 "/Game/Object/animal/material/cotton_animal_material.cotton_animal_material")))))

(event EventDoveDollHitSound
  (AddComponent|AddAudioComponent false))

(event EventDoveDollDeathSound
  (AddComponent|AddAudioComponent false))

(event EventSpawnParticle
  (bind _returnvalue (Effects|SpawnEmitteratLocation "/Game/VFX_Pack/Effects/monster_appears.monster_appears" (Transformation|GetWorldLocation (Variables|Character|GetMesh)) "0, 0, 0" "0.200000,0.200000,0.200000"))
  (Utilities|FlowControl|Delay 1.0)
  (Components|DestroyComponent _returnvalue))

(fn ConstructionScript)