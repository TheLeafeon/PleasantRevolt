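; Monster projectile actor that damages the player on impact and has a short lifespan set at BeginPlay, when its FireBall trail also starts.
; Any hit hides the actor; a hit on the player character applies FirePower as damage.
; Other hits reset the lifespan, spawn a scaled-down impact emitter at the collision component, and destroy that emitter after a delay that fits within the new lifespan.
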(event EventBeginPlay
  ;[1 1 1] 투사체 수명
  (Actor|SetLifeSpan 1.0)
  (Effects|Particles|Trails|BeginTrails (Variables|Default|GetFireBall) "None" "None" "ETrailWidthMode_FromCentre" 1.0))

(event Collision|EventHit
  (params (MyComp :type Primitive%20Component%20Object%20Reference) (Other :type Actor%20Object%20Reference) (OtherComp :type Primitive%20Component%20Object%20Reference) (bSelfMoved :type Boolean) (HitLocation :type Vector :default "0, 0, 0") (HitNormal :type Vector :default "0, 0, 0") (NormalImpulse :type Vector :default "0, 0, 0") (Hit :type Hit%20Result%20Structure%20%28by%20ref%29))
  ;[1 1 1] Hit
  (Rendering|SetActorHiddenInGame true)
  (if (== Other (Game|GetPlayerCharacter 0))
    (bind _asbp_playerable_character (Utilities|Casting|CastToBP_PlayerableCharacter Other))
    (Game|Damage|ApplyDamage _asbp_playerable_character (Variables|Default|GetFire_Power) 0 0)
    (Development|PrintString "Hit")
    (else
      (Actor|SetLifeSpan 1.1)
      (Development|PrintString "Not Player")
      (CallFunction|HitParticle)
      (Utilities|FlowControl|Delay 1.0)
      (Components|DestroyComponent (Variables|Default|GetMushroomParticle)))))

(fn ConstructionScript)

(fn HitParticle
  (bind _returnvalue (Effects|SpawnEmitteratLocation "/Game/VFX_Pack/Effects/Dove_ef_cr.Dove_ef_cr" (Transformation|GetWorldLocation (Variables|Default|GetCollisionComponent)) "0, 0, 0" "0.100000,0.100000,0.100000"))
  (Variables|Default|SetMushroomParticle _returnvalue))