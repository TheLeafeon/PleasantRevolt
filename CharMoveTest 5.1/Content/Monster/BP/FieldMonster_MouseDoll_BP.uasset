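; Field monster character for the MouseDoll, providing custom events for movement, attack, hit reaction and death against player 0.
; Attack events apply MonsterPower damage and spawn a short-lived impact emitter, while movement uses AIMoveTo toward the player.
; Knockback launches it away from the player; the death version launches harder, sets the AnimBP death flag and pauses the behavior tree.
; Hit feedback, skipped when dead, swaps three material slots to a hit material, blinks HitParam, then restores them.
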(event EventMouseDollApplyDamageEvent
  ;[1 1 1] 데미지 주기
  (bind _asbp_playerable_character (Utilities|Casting|CastToBP_PlayerableCharacter (Game|GetPlayerCharacter 0)))
  (Game|Damage|ApplyDamage _asbp_playerable_character (Variables|Default|GetMonster_Power) 0 0))

(event EventMouseDollHitMaterial
  ;[1 1 1] 흰색[길게] 시간 - 빨/기존 메쉬[깜빡] 횟수
  (if (not (Variables|Default|GetisDie))
    (Utilities|FlowControl|Sequence
      (:then_0
        ;;[1 1 1] 흰색 길게
        (Rendering|Material|SetMaterial (Variables|Character|GetMesh) 0 "/Game/Monster/Material/FieldMonster_material_Hit.FieldMonster_material_Hit")
        (Utilities|FlowControl|Delay 0.3)
        ;;[1 1 1] 빨간색 깜빡
        (Rendering|Material|SetScalarParameterValueonMaterials (Variables|Character|GetMesh) "HitParam" 0.0)
        (Utilities|FlowControl|Delay 0.1)
        (Rendering|Material|SetScalarParameterValueonMaterials (Variables|Character|GetMesh) "HitParam" 1.0)
        (Utilities|FlowControl|Delay 0.1)
        (Rendering|Material|SetMaterial (Variables|Character|GetMesh) 0 "/Game/Object/animal/material/mouse_material.mouse_material"))
      (:then_1
        (Rendering|Material|SetMaterial (Variables|Character|GetMesh) 1 "/Game/Monster/Material/FieldMonster_material_Hit.FieldMonster_material_Hit")
        (Utilities|FlowControl|Delay 0.3)
        (Rendering|Material|SetScalarParameterValueonMaterials (Variables|Character|GetMesh) "HitParam" 0.0)
        (Utilities|FlowControl|Delay 0.1)
        (Rendering|Material|SetScalarParameterValueonMaterials (Variables|Character|GetMesh) "HitParam" 1.0)
        (Utilities|FlowControl|Delay 0.1)
        (Rendering|Material|SetMaterial (Variables|Character|GetMesh) 1 "/Game/Object/animal/material/mouse_material.mouse_material"))
      (:then_2
        (Rendering|Material|SetMaterial (Variables|Character|GetMesh) 2 "/Game/Monster/Material/FieldMonster_material_Hit.FieldMonster_material_Hit")
        (Utilities|FlowControl|Delay 0.3)
        (Rendering|Material|SetScalarParameterValueonMaterials (Variables|Character|GetMesh) "HitParam" 0.0)
        (Utilities|FlowControl|Delay 0.1)
        (Rendering|Material|SetScalarParameterValueonMaterials (Variables|Character|GetMesh) "HitParam" 1.0)
        (Utilities|FlowControl|Delay 0.1)
        (Rendering|Material|SetMaterial (Variables|Character|GetMesh) 2 "/Game/Object/animal/material/mouse_material.mouse_material")))))

(event EventMouseDollAttackParticle
  ;[1 1 1] 파티클 출력
  (bind _returnvalue (Effects|SpawnEmitteratLocation "/Game/buy_asset/VFX_Pack/Effects/P_Impact_03.P_Impact_03" (Transformation|GetWorldLocation (Variables|Default|GetAttackParticlePoint)) "0, 0, 0" "0.200000,0.200000,0.200000"))
  (Utilities|FlowControl|Delay 1.0)
  (Components|DestroyComponent _returnvalue))

(event EventMouseDollKnockBack
  ;[1 1 1] 넉백
  (Character|LaunchCharacter (* (Math|Vector|GetUnitDirection(Vector) (Transformation|GetActorLocation (Game|GetPlayerCharacter 0)) (Transformation|GetActorLocation)) (Math|Conversions|ToVector(Float) 1e+03)) false false))

(event EventMouseDollDeathKnockBack
  ;[1 1 1] 죽었을때 더 멀리 날라가게
  (Character|LaunchCharacter (* (Math|Vector|GetUnitDirection(Vector) (Transformation|GetActorLocation (Game|GetPlayerCharacter 0)) (Transformation|GetActorLocation)) (Math|Conversions|ToVector(Float) 6e+03)) false false)
  (bind _asmouse_doll_anim_bp (Utilities|Casting|CastToMouseDollAnim_BP (Components|SkeletalMesh|GetAnimInstance (Variables|Character|GetMesh))))
  (Variables|/Game/Monster/Animation/AnimBP/MouseDollAnim_BP.MouseDollAnim_BP_C|SetisDeath? _asmouse_doll_anim_bp true)
  (bind _asmouse_doll_aicontroller (Utilities|Casting|CastToMouseDollAIController (Pawn|GetController)))
  (Class|MouseDollAIController|PauseBehaviorTree _asmouse_doll_aicontroller))

(event EventMouseDollMovetoTarget
  (AI|AIMoveTo self "0, 0, 0" (Game|GetPlayerCharacter 0) 5.0 false))

(fn ConstructionScript)