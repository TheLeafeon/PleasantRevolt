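; FieldMonster_RabbitDoll is a field monster that hops in place and damages the player when they touch its attack box.
; Tick waits on a short Delay, then alternates Jumping and Landing timelines, toggled by IsLanding, that add vertical offsets to the static mesh.
; RabbitDollKnockBack launches the doll away from the player.
; Overlap with AttackRangeBox applies MonsterPower damage to the player character.
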(event OnComponentBeginOverlap(AttackRangeBox)
  (params (OverlappedComponent :type Primitive%20Component%20Object%20Reference) (OtherActor :type Actor%20Object%20Reference) (OtherComp :type Primitive%20Component%20Object%20Reference) (OtherBodyIndex :type Integer) (bFromSweep :type Boolean) (SweepResult :type Hit%20Result%20Structure%20%28by%20ref%29))
  (bind _returnvalue (Game|GetPlayerCharacter 0))
  ;[1 1 1] ApplyDamage
  (if (== OtherActor _returnvalue)
    (bind _asbp_playerable_character (Utilities|Casting|CastToBP_PlayerableCharacter _returnvalue))
    (Game|Damage|ApplyDamage _asbp_playerable_character (Variables|Default|GetMonster_Power) 0 0)))

(event EventRabbitDollKnockBack
  ;[1 1 1] RabbitDoll KnockBack
  (Character|LaunchCharacter (* (Math|Vector|GetUnitDirection(Vector) (Transformation|GetActorLocation (Game|GetPlayerCharacter 0)) (Transformation|GetActorLocation)) (Math|Conversions|ToVector(Float) 1e+05)) false false))

(event Collision|EventHit
  (params (MyComp :type Primitive%20Component%20Object%20Reference) (Other :type Actor%20Object%20Reference) (OtherComp :type Primitive%20Component%20Object%20Reference) (bSelfMoved :type Boolean) (HitLocation :type Vector :default "0, 0, 0") (HitNormal :type Vector :default "0, 0, 0") (NormalImpulse :type Vector :default "0, 0, 0") (Hit :type Hit%20Result%20Structure%20%28by%20ref%29)))

(event EventTick
  (params (DeltaSeconds :type Float%20%28single-precision%29))
  ;[1 1 1] 점프
  (Utilities|FlowControl|Delay 0.21)
  (if (Variables|Default|GetisLanding?)
    (bind _jumping (Timeline|JumpingTimeLine PlayFromStart)
      (:Update
        (Transformation|AddLocalOffset (Variables|Default|GetStaticMesh) (Math|Vector|MakeVector 0.0 0.0 _jumping) false false)
        (Variables|Default|SetisLanding? false)))
    (else
      (bind _landing (Timeline|LandingTimeLine PlayFromStart)
        (:Update
          (Transformation|AddLocalOffset (Variables|Default|GetStaticMesh) (Math|Vector|MakeVector 0.0 0.0 _landing) false false)
          (Variables|Default|SetisLanding? true))))))

(fn ConstructionScript)