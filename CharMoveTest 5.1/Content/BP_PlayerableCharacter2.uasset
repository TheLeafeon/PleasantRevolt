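; Player character with a cable grappling hook, a melee attack montage, a health HUD and debug keys that damage or heal it.
; Right-click line-traces toward the deprojected mouse position at mesh height to set a hook point, or launches the character toward an existing one.
; Tick interpolates the Cable component to the hook, fixes its length once attached, and releases it when the player's distance leaves that length's tolerance band.
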(event Custom|StopGrapple
  (bind _cable (Variables|Default|GetCable))
  (bind _cable_2 (Variables|Default|GetCable))
  (Variables|Default|SetHooked false)
  (Variables|Default|SetHook%20Move%20Finished false)
  (Rendering|SetVisibility _cable_2 false false)
  (Transformation|SetWorldLocation _cable_2 (Transformation|GetActorLocation) false false)
  (Utilities|FlowControl|DoOnce false) ; enters at Reset
)

(event Custom|MovePlayerToGrappling
  (CallFunction|MovePlayer)
  (Variables|/Script/CableComponent.CableComponent|SetCableLength (Variables|Default|GetCable) (Math|Vector|VectorLength (- (Transformation|GetActorLocation) (Variables|Default|GetHook%20Location)))))

(event EventBeginPlay
  (bind _cable (Variables|Default|GetCable))
  (bind _returnvalue (UserInterface|CreateWidget "/Game/PlayerTest/Player/Player_UMG/UMG_PlayerHealth.UMG_PlayerHealth_C" (Game|GetPlayerController 0)))
  (UserInterface|Viewport|AddtoViewport _returnvalue 0)
  ;[1 1 1] 코멘트
  (Rendering|SetVisibility _cable false false)
  (Variables|/Script/CableComponent.CableComponent|SetCableLength _cable 0.0)
  (Variables|/Script/CableComponent.CableComponent|SetCableWidth _cable 2.0)
  (Variables|/Script/CableComponent.CableComponent|SetEndLocation _cable "30.000000,0.000000,0.000000"))

(event EventTick
  (params (DeltaSeconds :type Float%20%28single-precision%29))
  (bind _returnvalue (Transformation|GetActorLocation))
  (bind _cable (Variables|Default|GetCable))
  (bind _hook_location (Variables|Default|GetHook%20Location))
  (bind _cable_2 (Variables|Default|GetCable))
  (bind _returnvalue_2 (- _returnvalue _hook_location))
  (bind _returnvalue_3 (Math|Vector|VectorLength _returnvalue_2))
  (if (Variables|Default|GetHooked)
    (if (Variables|Default|GetHook%20Move%20Finished)
      (Utilities|FlowControl|Sequence
        (:then_0
          (Transformation|SetWorldLocationAndRotation _cable_2 (Math|Interpolation|VInterpTo (Transformation|GetWorldLocation _cable_2) (Variables|Default|GetHook%20Location) (Utilities|Time|GetWorldDeltaSeconds) 2.5e+02) (Math|Rotator|FindLookatRotation (Transformation|GetActorLocation) (Variables|Default|GetHook%20Location)) false false)
          (Utilities|FlowControl|DoOnce false
            (:Completed
              (bind _output_get (Variables|/Script/CableComponent.CableComponent|SetCableLength _cable (+ (Math|Vector|VectorLength (- (Transformation|GetActorLocation) (Variables|Default|GetHook%20Location))) 5e+01)))
              (Variables|Default|SetNewCableLength _output_get)
              (Variables|/Script/CableComponent.CableComponent|SetEndLocation _cable "15.000000,0.000000,30.000000"))))
        (:then_1
          (if (or (>= _returnvalue_3 (+ (Variables|Default|GetNewCableLength) 4e+02)) (<= _returnvalue_3 (- (Variables|Default|GetNewCableLength) 3e+02)))
            (CallFunction|StopGrapple))))
      (else
        (bind _reached_location (CallFunction|MoveCable))
        (Variables|Default|SetHook%20Move%20Finished _reached_location)))))

(event Input|KeyboardEvents|3
  (params (Key :type Key%20Structure :default "None"))
  (:Pressed
    (Game|Damage|ApplyDamage self 1.0 0 0)
    (bind _returnvalue (Class|PlayerableCharacter|GetPlayerHP))
    (Development|PrintText (Utilities|Text|ToText(Float) _returnvalue "HalfToEven"))))

(event Input|MouseEvents|RightMouseButton
  (params (Key :type Key%20Structure :default "None"))
  (bind _returnvalue (Game|GetPlayerController 0))
  (bind _mesh (Variables|Character|GetMesh))
  (bind _worldlocation (Game|Player|ConvertMouseLocationToWorldSpace _returnvalue))
  (:Pressed
    (if (Variables|Default|GetHooked)
      (CallFunction|MovePlayertoGrappling)
      (else
        (bind (_outhit _returnvalue_2) (Collision|LineTraceForObjects (Transformation|GetWorldLocation _mesh) (Math|Vector|MakeVector (.x _worldlocation) (.y _worldlocation) (.z (Transformation|GetWorldLocation _mesh))) (Utilities|Array|MakeArray "ObjectTypeQuery1" "ObjectTypeQuery2") false 0 "Persistent"))
        (if _returnvalue_2
          (Transformation|SetActorRotation (Math|Rotator|MakeRotator 0.0 0.0 (.yaw (Math|Rotator|FindLookatRotation (Transformation|GetActorLocation) (.Location (Collision|BreakHitResult _outhit))))))
          (Variables|Default|SetHooked true)
          (Variables|Default|SetHook%20Location (.Location (Collision|BreakHitResult _outhit)))
          (else
            (CallFunction|StopGrapple)))))))

(event Input|KeyboardEvents|4
  (params (Key :type Key%20Structure :default "None"))
  (:Pressed
    (Class|PlayerableCharacter|IncreasePlayerHP 1.0)
    (bind _returnvalue (Class|PlayerableCharacter|GetPlayerHP))
    (Development|PrintText (Utilities|Text|ToText(Float) _returnvalue "HalfToEven"))))

(event Input|KeyboardEvents|C
  (params (Key :type Key%20Structure :default "None"))
  (:Pressed
    (Animation|PlayAnimMontage "/Game/PlayerTest/Player/Animations/NearWeapon3_Attack_Montage.NearWeapon3_Attack_Montage" 1.0 "None")))

(fn ConstructionScript)

(fn MoveCable
  (bind _cable (Variables|Default|GetCable))
  (bind _hook_location (Variables|Default|GetHook%20Location))
  (bind _returnvalue (Transformation|GetWorldLocation _cable))
  (Rendering|SetVisibility _cable true false)
  (if (<= (Math|Vector|VectorLength (- _returnvalue _hook_location)) 1e+02)
    (return true)
    (else
      (Transformation|SetWorldLocation _cable (Math|Interpolation|VInterpTo _returnvalue _hook_location (Utilities|Time|GetWorldDeltaSeconds) 0.0) false false)
      (return false))))

(fn MovePlayer
  (Character|LaunchCharacter (* (- (Variables|Default|GetHook%20Location) (Transformation|GetActorLocation (Game|Player|GetPlayerPawn 0))) (* (Utilities|Time|GetWorldDeltaSeconds) 2.5e+02)) true true))