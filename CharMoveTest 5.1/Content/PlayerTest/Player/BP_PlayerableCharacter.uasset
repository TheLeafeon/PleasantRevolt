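; BP_PlayerableCharacter is a player character Blueprint that shows a health HUD and tests HP changes and a melee combo animation.
; BeginPlay creates the UMG_PlayerHealth widget for the first player controller and adds it to the viewport.
; Right mouse plays the near-weapon combo montage.
; Number-key debug inputs heal through IncreasePlayerHP or damage the character through ApplyDamage, then both print the current HP.
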(event EventBeginPlay
  (bind _returnvalue (UserInterface|CreateWidget "/Game/PlayerTest/Player/Player_UMG/UMG_PlayerHealth.UMG_PlayerHealth_C" (Game|GetPlayerController 0)))
  (UserInterface|Viewport|AddtoViewport _returnvalue 0))

(event Input|KeyboardEvents|3
  (params (Key :type Key%20Structure :default "None"))
  (:Pressed
    (Game|Damage|ApplyDamage self 1.0 0 0)
    (bind _returnvalue (Class|PlayerableCharacter|GetPlayerHP))
    (Development|PrintText (Utilities|Text|ToText(Float) _returnvalue "HalfToEven"))))

(event Input|MouseEvents|RightMouseButton
  (params (Key :type Key%20Structure :default "None"))
  (:Pressed
    (Animation|PlayAnimMontage "/Game/PlayerTest/Player/Animations/Nearweapon1_Combo_Montage.Nearweapon1_Combo_Montage" 1.0 "None")))

(event Input|KeyboardEvents|4
  (params (Key :type Key%20Structure :default "None"))
  (:Pressed
    (Class|PlayerableCharacter|IncreasePlayerHP 1.0)
    (bind _returnvalue (Class|PlayerableCharacter|GetPlayerHP))
    (Development|PrintText (Utilities|Text|ToText(Float) _returnvalue "HalfToEven"))))

(fn ConstructionScript)